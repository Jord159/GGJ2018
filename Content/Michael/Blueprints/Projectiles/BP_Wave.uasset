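; BP_Wave is a projectile Blueprint for a wave that changes size over its lifetime.
; Each Tick multiplies all three scale axes by Coeff while keeping location and rotation, so the size change compounds per frame, independent of delta time.
; On overlap it destroys itself unless the other actor carries the Wave or Receiver tag, letting it pass through other waves and receivers.
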(event EventTick
  (params (DeltaSeconds :type Float%20%28single-precision%29))
  (bind _returnvalue (Transformation|GetActorTransform))
  (bind _coeff (Variables|Default|Getcoeff))
  (bind (_location _rotation _scale) (Math|Transform|BreakTransform _returnvalue))
  (bind (_x _y _z) (Math|Vector|BreakVector _scale))
  (Transformation|SetActorTransform (Math|Transform|MakeTransform _location _rotation (Math|Vector|MakeVector (* _x _coeff) (* _y _coeff) (* _z _coeff)))))

(event Collision|EventActorBeginOverlap
  (params (OtherActor :type Actor%20Object%20Reference))
  (if (Math|Boolean|NORBoolean (Actor|ActorHasTag OtherActor "Wave") (Actor|ActorHasTag OtherActor "Receiver"))
    (Actor|DestroyActor)))

(fn ConstructionScript)