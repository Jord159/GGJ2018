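; BP_Receiver is a pawn that drifts randomly and checks the color of waves that hit it.
; A looping timer picks a new random X/Z movement vector, which Tick feeds to the floating pawn movement component.
; On overlap with a Wave-tagged BP_Wave, it compares the plane's material to its accepted material, prints a debug GOOD or BAD, and destroys the wave.
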(event Collision|EventActorBeginOverlap
  (params (OtherActor :type Actor%20Object%20Reference))
  ;[0 0 0] On collision with wave print string to see if valid color
  (Utilities|IsValid OtherActor
    (:Is%20Valid
      (if (Actor|ActorHasTag OtherActor "Wave")
        (bind _asbp_wave (Utilities|Casting|CastToBP_Wave OtherActor))
        (if (== (Rendering|Material|GetMaterial (Variables|/Game/Michael/Blueprints/Projectiles/BP_Wave.BP_Wave_C|GetPlane _asbp_wave) 0) (Variables|Default|GetAcceptedMaterial))
          (Development|PrintString "GOOD") ; Print debug string
          (else
            (Development|PrintString "BAD") ; Print debug string
          ))
        (Actor|DestroyActor OtherActor)))))

(event EventBeginPlay
  (CallFunction|ChangeDirection)
  (Utilities|Time|SetTimerbyFunctionName 0 "ChangeDirection" (Variables|Default|GetTimer) true))

(event EventTick
  (params (DeltaSeconds :type Float%20%28single-precision%29))
  ;[0 0 0] Update movement vector every frame
  (Class|PawnMovementComponent|AddInputVector (Variables|Default|GetFloatingPawnMovement) (Variables|Default|GetMovementVector) false))

(fn ConstructionScript)

(fn ChangeDirection
  (Variables|Default|SetMovementVector (Math|Vector|MakeVector (Math|Random|RandomFloatinRange (Variables|Default|GetMinX) (Variables|Default|GetMaxX)) 0.0 (Math|Random|RandomFloatinRange (Variables|Default|GetMinZ) (Variables|Default|GetMaxZ)))))