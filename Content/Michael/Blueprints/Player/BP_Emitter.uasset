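; BP_Emitter is a player-controlled actor that continuously fires coloured waves.
; A looping timer from BeginPlay calls SpawnWave, which spawns a WaveClass actor at the emitter's Plane using its rotation and applies the selected material.
; ColourUp and ColourDown inputs cycle through three colour indices with wraparound.
; The EmitterMovement axis adjusts the emitter's pitch within a clamped range, aiming subsequent waves.
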(event EventBeginPlay
  (Utilities|Time|SetTimerbyFunctionName 0 "SpawnWave" (/ (/ 128.0 6e+01) 15.0) true))

(event Input|ActionEvents|InputActionColourUp
  (params (Key :type Key%20Structure))
  (:Pressed
    (if (> (+ (Variables|Default|GetWaveColourIndex) 1) 2)
      (Variables|Default|SetWaveColourIndex 0)
      (else
        (Variables|Default|SetWaveColourIndex (+ (Variables|Default|GetWaveColourIndex) 1))))))

(event Input|ActionEvents|InputActionColourDown
  (params (Key :type Key%20Structure))
  (:Pressed
    (if (< (- (Variables|Default|GetWaveColourIndex) 1) 0)
      (Variables|Default|SetWaveColourIndex 2)
      (else
        (Variables|Default|SetWaveColourIndex (- (Variables|Default|GetWaveColourIndex) 1))))))

(event Input|AxisEvents|InputAxisEmitterMovement
  (params (AxisValue :type Float%20%28single-precision%29))
  (bind _returnvalue (Transformation|GetActorRotation))
  (Transformation|SetActorRotation (Math|Rotator|MakeRotator (.roll _returnvalue) (Math|Float|Clamp(Float) (+ AxisValue (.pitch _returnvalue)) -45.0 45.0) (.yaw _returnvalue))))

(fn ConstructionScript)

(fn SpawnWave
  (bind _returnvalue (Game|SpawnActorfromClass (Variables|Default|GetWaveClass) (Math|Transform|MakeTransform (Transformation|GetWorldLocation (Variables|Default|GetPlane)) (Transformation|GetActorRotation) "2.000000,2.000000,2.000000") "Undefined" 0 0))
  (Utilities|IsValid _returnvalue
    (:Is%20Valid
      (Rendering|Material|SetMaterial (Variables|/Game/Michael/Blueprints/Projectiles/BP_Wave.BP_Wave_C|GetPlane _returnvalue) 0 (Utilities|Array|Get(acopy) (Variables|Default|GetWaveMaterials) (Variables|Default|GetWaveColourIndex))))))