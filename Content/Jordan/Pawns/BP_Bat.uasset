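; Bat pawn that flies toward a hard-coded world point.
; BeginPlay snaps DummyRoot to the start of the spline on its SplineBP reference.
; Each Tick, until it is at the target, it turns to face it and feeds the offset into FloatingPawnMovement.
; A looping spline-follow path in Tick is switched off by a constant false branch.
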(event EventBeginPlay
  (Variables|Default|SetSpline%20Dist 0.0)
  (Transformation|SetWorldLocation (Variables|Default|GetDummyRoot) (Spline|GetLocationatDistanceAlongSpline (Variables|/Game/Jordan/Splines/Figure8.Figure8_C|GetSpline (Variables|Default|GetSplineBP)) (Variables|Default|GetSpline%20Dist) "World") false false))

(event EventTick
  (params (DeltaSeconds :type Float%20%28single-precision%29))
  (bind _returnvalue (Transformation|GetActorLocation))
  (bind _returnvalue_2 (Math|Vector|MakeVector 1.65e+03 0.0 8e+02))
  (bind _splinebp (Variables|Default|GetSplineBP))
  (bind _spline (Variables|/Game/Jordan/Splines/Figure8.Figure8_C|GetSpline _splinebp))
  (if false
    (bind _result (Math|Float|IncrementFloat (Variables|Default|GetSpline%20Dist))
      (:%20%20
        (Transformation|SetWorldLocation (Variables|Default|GetDummyRoot) (Spline|GetLocationatDistanceAlongSpline _spline (Math|Float|%(Float) _result (Spline|GetSplineLength _spline)) "World") false false)))
    (elif (not (Math|Vector|Equal(Vector) _returnvalue _returnvalue_2 0.1))
      (Transformation|SetActorRotation (Math|Rotator|FindLookatRotation _returnvalue _returnvalue_2) true)
      (Class|PawnMovementComponent|AddInputVector (Variables|Default|GetFloatingPawnMovement) (- _returnvalue_2 _returnvalue) false))))

(fn ConstructionScript)